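; Ship projectile actor that damages enemy ships on contact.
; On BeginPlay its Sphere component ignores the instigator when moving, so it does not collide with the shooter.
; A Sphere overlap with a BP_EnemyShip applies BaseDamage credited to the instigator's controller, then calls CleanUp to destroy the projectile.
; Overlaps with any other actor have no effect.
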(event `self.ReceiveBeginPlay`
  (`PrimitiveComponent.IgnoreActorWhenMoving` (`self.Sphere`) (`self.GetInstigator`) true))

(event `self.ReceiveTick`
  (params (DeltaSeconds :type "Float (single-precision)")))

(event `self.Sphere.OnComponentBeginOverlap`
  (params (OverlappedComponent :type "PrimitiveComponent Object Reference") (OtherActor :type "Actor Object Reference") (OtherComp :type "PrimitiveComponent Object Reference") (OtherBodyIndex :type Integer) (bFromSweep :type Boolean) (SweepResult :type "HitResult Structure (by ref)"))
  (bind _asbp_enemy_ship (cast `/Game/Blueprints/Ships/BP_EnemyShip` OtherActor))
  (`GameplayStatics.ApplyDamage` _asbp_enemy_ship (`self.BaseDamage`) (`self.GetInstigatorController`) self)
  (`self.CleanUp`))

(fn `CleanUp`
  (`self.K2_DestroyActor`))

(fn `UserConstructionScript`)