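; Player ship that constantly flies forward along its facing, speeding up by a multiplier on a looping timer.
; Overlapping an enemy ship reports death to PC_ShipController, which also receives enemy kill events.
; Shot cooldown power-ups scale the cooldown duration, then a delay restores the base value cached in the construction script and cleans up the power-up.
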(event `self.ReceiveBeginPlay`
  (`KismetSystemLibrary.Delay` (`self.SpeedIncreaseInterval`))
  (`KismetSystemLibrary.K2_SetTimer` null "IncreaseMovementSpeed" (`self.SpeedIncreaseInterval`) true))

(event `self.ReceiveActorBeginOverlap`
  (params (OtherActor :type "Actor Object Reference"))
  (cast `/Game/Actors/Ships/BP_EnemyShip` OtherActor)
  (bind _aspc_ship_controller (cast `/Game/Core/Controllers/PC_ShipController` (`self.GetController`)))
  (`/Game/Core/Controllers/PC_ShipController.OnDeath` _aspc_ship_controller))

(event `self.ReceiveTick`
  (params (DeltaSeconds :type "Float (single-precision)"))
  (`self.K2_SetActorLocation` (+ (`self.K2_GetActorLocation`) (* (`self.GetActorForwardVector`) (* DeltaSeconds (`self.MovementSpeed`))))))

(event `OnEnemyKill`
  (bind _aspc_ship_controller (cast `/Game/Core/Controllers/PC_ShipController` (`self.GetController`)))
  (`/Game/Core/Controllers/PC_ShipController.OnEnemyKill` _aspc_ship_controller))

(event `OnPowerUpApplied`
  (params (PowerUp :type "/Game/Core/PowerUps/BP_BasePowerUp Object Reference"))
  (`KismetSystemLibrary.Delay` (`BasePowerUp.EffectDuration` PowerUp))
  (`self.RemovePowerUp` PowerUp))

(fn `ApplyPowerUp`
  (params (PowerUp :type "/Game/Core/PowerUps/BP_BasePowerUp Object Reference"))
  (switch `PowerUpType` (`BasePowerUp.Type` PowerUp)
    (:`FasterShotCoolDown`
      (bind _asbp_shot_cool_down_pu (cast `/Game/Actors/PowerUps/BP_ShotCoolDownPU` PowerUp))
      (set `self.CoolDownDuration` (* (`/Game/Actors/PowerUps/BP_ShotCoolDownPU.CoolDownDurationMultiplier` _asbp_shot_cool_down_pu) (`self.CoolDownDuration`)))
      (`self.OnPowerUpApplied` (`local.PowerUp`)))))

(fn `IncreaseMovementSpeed`
  (set `self.MovementSpeed` (* (`self.MovementSpeed`) (`self.MovementSpeedMultiplier`))))

(fn `RemovePowerUp`
  (params (PowerUp :type "/Game/Core/PowerUps/BP_BasePowerUp Object Reference"))
  (switch `PowerUpType` (`BasePowerUp.Type` PowerUp)
    (:`FasterShotCoolDown`
      (set `self.CoolDownDuration` (`self.BaseShotCoolDownDuration`))
      (`/Game/Core/PowerUps/BP_BasePowerUp.CleanUp` (`local.PowerUp`)))))

(fn `UserConstructionScript`
  (`parent.UserConstructionScript`)
  (`self.K2_SetActorRotation` (struct))
  (set `self.BaseShotCoolDownDuration` (`self.CoolDownDuration`)))