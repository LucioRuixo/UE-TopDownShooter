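; Auto-scrolling player camera actor that moves steadily along a set direction and gradually speeds up during play.
; Tick advances it without sweeping, while a looping timer, started after an initial delay, compounds the speed by a multiplier.
; Its collider tells overlapping enemy ships they are off-screen and triggers death on the ship controller when the player ship overlaps it.
; Construction resets rotation and applies the camera's Z offset.
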(event `self.ReceiveBeginPlay`
  (`KismetSystemLibrary.Delay` (`self.SpeedIncreaseInterval`))
  (`KismetSystemLibrary.K2_SetTimer` null "IncreaseMovementSpeed" (`self.SpeedIncreaseInterval`) true))

(event `self.Collider.OnComponentBeginOverlap`
  (params (OverlappedComponent :type "PrimitiveComponent Object Reference") (OtherActor :type "Actor Object Reference") (OtherComp :type "PrimitiveComponent Object Reference") (OtherBodyIndex :type Integer) (bFromSweep :type Boolean) (SweepResult :type "HitResult Structure (by ref)"))
  (bind _asbp_enemy_ship (cast `/Game/Actors/Ships/BP_EnemyShip` OtherActor)
    (:`then`
      (`/Game/Actors/Ships/BP_EnemyShip.OnOffScreen` _asbp_enemy_ship))
    (:`CastFailed`
      (cast `/Game/Actors/Ships/BP_PlayerShip` OtherActor)
      (bind _aspc_ship_controller (cast `/Game/Core/Controllers/PC_ShipController` (`GameplayStatics.GetPlayerController` 0)))
      (`/Game/Core/Controllers/PC_ShipController.OnDeath` _aspc_ship_controller))))

(event `self.ReceiveTick`
  (params (DeltaSeconds :type "Float (single-precision)"))
  (`self.K2_SetActorLocation` (+ (`self.K2_GetActorLocation`) (* (`self.MovementDirection`) (* DeltaSeconds (`self.MovementSpeed`))))))

(fn `IncreaseMovementSpeed`
  (set `self.MovementSpeed` (* (`self.MovementSpeed`) (`self.MovementSpeedMultiplier`))))

(fn `UserConstructionScript`
  (`self.K2_SetActorRotation` (struct))
  (`SceneComponent.K2_SetRelativeLocation` (`self.Camera`) (`KismetMathLibrary.MakeVector` 0.0 0.0 (`self.LocationZ`)) false false))