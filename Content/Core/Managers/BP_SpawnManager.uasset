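; Spawn manager that spawns enemy ships and random power-ups ahead of the player camera during gameplay.
; StartSpawning sets two looping timers, each interval randomized only once at start; StopSpawning clears only the enemy timer.
; GetSpawnTransform offsets from the GM_Gameplay camera by a forward distance and random lateral spread, using player pawn height and a fixed 180-degree rotation.
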(event `StartSpawning`
  (bind _returnvalue (`KismetSystemLibrary.K2_SetTimer` null "SpawnEnemy" (`KismetMathLibrary.RandomFloatInRange` (`self.EnemyMinSpawnTime`) (`self.EnemyMaxSpawnTime`)) true))
  (set `self.EnemySpawnTimer` _returnvalue)
  (bind _returnvalue_2 (`KismetSystemLibrary.K2_SetTimer` null "SpawnPowerUp" (`KismetMathLibrary.RandomFloatInRange` (`self.PowerUpMinSpawnTime`) (`self.PowerUpMaxSpawnTime`)) true))
  (set `self.PowerUpSpawnTimer` _returnvalue_2))

(event `StopSpawning`
  (`KismetSystemLibrary.K2_ClearAndInvalidateTimerHandle` (`self.EnemySpawnTimer`)))

(fn `GetSpawnTransform`
  (returns (Transform :type "Transform Structure"))
  (bind _spawnmaxlateraldistance (`self.SpawnMaxLateralDistance`))
  (bind (_returnvalue_x _returnvalue_y _returnvalue_z) (`KismetMathLibrary.BreakVector` (`self.K2_GetActorLocation` (`GameplayStatics.GetPlayerPawn` 0))))
  (bind _asgm_gameplay (cast `/Game/Core/GameModes/GM_Gameplay` (`GameplayStatics.GetGameMode`)))
  (bind _playercamera (`/Game/Core/GameModes/GM_Gameplay.PlayerCamera` _asgm_gameplay))
  (bind (_returnvalue_x_2 _returnvalue_y_2) (`KismetMathLibrary.BreakVector` (+ (`self.K2_GetActorLocation` _playercamera) (* (`self.GetActorRightVector` _playercamera) (`KismetMathLibrary.RandomFloatInRange` (* _spawnmaxlateraldistance -1.0) _spawnmaxlateraldistance)) (* (`self.GetActorForwardVector` _playercamera) (`self.SpawnForwardDistance`)))))
  (return (`KismetMathLibrary.MakeTransform` (`KismetMathLibrary.MakeVector` _returnvalue_x_2 _returnvalue_y_2 _returnvalue_z) (struct :`Yaw` 180.0))))

(fn `SpawnEnemy`
  (`|SpawnActorFromClass` "/Game/Blueprints/Ships/BP_EnemyShip.BP_EnemyShip_C" (`self.GetSpawnTransform`) "Undefined" "OverrideRootScale" null null))

(fn `SpawnPowerUp`
  (bind _powerupclasses (`self.PowerUpClasses`))
  (`|SpawnActorFromClass` (`|GetArrayItem` _powerupclasses (`KismetMathLibrary.RandomIntegerInRange` 0 (- (`KismetArrayLibrary.Array_Length` _powerupclasses) 1))) (`self.GetSpawnTransform`) "AlwaysSpawn" "OverrideRootScale" null null))

(fn `UserConstructionScript`)