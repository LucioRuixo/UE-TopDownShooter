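; PC_ShipController is a controller that tracks the player's score and relays ship gameplay events to the HUD and game mode.
; OnEnemyKill adds KillScoreAddition to Score and pushes the new total to BP_HUD through UpdateScore.
; OnDeath forwards the death to GM_Gameplay by calling OnPlayerDeath.
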(event `OnEnemyKill`
  (bind _output_get (set `self.Score` (+ (`self.Score`) (`self.KillScoreAddition`))))
  (bind _asbp_hud (cast `/Game/UI/BP_HUD` (`self.GetHUD`)))
  (`/Game/UI/BP_HUD.UpdateScore` _asbp_hud _output_get))

(event `OnDeath`
  (bind _asgm_gameplay (cast `/Game/Core/GameModes/GM_Gameplay` (`GameplayStatics.GetGameMode`)))
  (`/Game/Core/GameModes/GM_Gameplay.OnPlayerDeath` _asgm_gameplay))

(fn `UserConstructionScript`)