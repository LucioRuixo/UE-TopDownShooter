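; Gameplay game mode that sets up the level, runs the start/end game flow and restarts on player death.
; BeginPlay moves the player pawn to the origin, spawns a player camera there as the view target, creates a spawn manager, then starts the game.
; Start and end game events switch spawning on and off.
; Player death ends the game and reloads the current level by name.
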(event `self.ReceiveBeginPlay`
  (`self.K2_SetActorLocation` (`GameplayStatics.GetPlayerPawn` 0) (0.0 0.0 0.0) false false)
  (`self.SetUpCamera`)
  (`self.SetUpSpawnManager`)
  (`self.StartGame`))

(event `self.OnStartGame`
  (`/Game/Core/Managers/BP_SpawnManager.StartSpawning` (`self.SpawnManager`)))

(event `self.OnEndGame`
  (`/Game/Core/Managers/BP_SpawnManager.StopSpawning` (`self.SpawnManager`)))

(event `OnPlayerDeath`
  (`self.EndGame`)
  (`KismetSystemLibrary.PrintString` "restarting level")
  (bind _returnvalue (`GameplayStatics.GetCurrentLevelName` true))
  (`GameplayStatics.OpenLevel` (`KismetStringLibrary.Conv_StringToName` _returnvalue)))

(fn `SetUpCamera`
  (`|ExecutionSequence`
    (:`then_0`
      ;[1 1 1] Create camera if necessary
      (if (not (`KismetSystemLibrary.IsValid` (`self.PlayerCamera`)))
        (bind _returnvalue (`|SpawnActorFromClass` "/Game/Core/Cameras/BP_PlayerCamera.BP_PlayerCamera_C" (`KismetMathLibrary.MakeTransform` (0.0 0.0 0.0)) "Undefined" "OverrideRootScale" null null))
        (set `self.PlayerCamera` _returnvalue)))
    (:`then_1`
      ;[1 1 1] Set location of camera
      (`self.K2_SetActorLocation` (`self.PlayerCamera`) (`self.K2_GetActorLocation` (`GameplayStatics.GetPlayerPawn` 0)) false false))
    (:`then_2`
      ;[1 1 1] Set new view target
      (`PlayerController.SetViewTargetWithBlend` (`GameplayStatics.GetPlayerController` 0) (`self.PlayerCamera`) 0.0 "VTBlend_Linear" 0.0 false))))

(fn `SetUpSpawnManager`
  (bind _returnvalue (`|SpawnActorFromClass` "/Game/Core/Managers/BP_SpawnManager.BP_SpawnManager_C" (`KismetMathLibrary.MakeTransform` (0.0 0.0 0.0)) "Undefined" "OverrideRootScale" null null))
  (set `self.SpawnManager` _returnvalue))

(fn `UserConstructionScript`)